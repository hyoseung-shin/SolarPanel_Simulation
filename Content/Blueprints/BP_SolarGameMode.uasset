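; BP_SolarGameMode is a game mode that sets up a solar simulation session when play begins.
; It starts recording on the SolarSimulationSubsystem, adds a solar HUD widget to the viewport, and spawns a solar panel actor at a fixed spot.
; The panel is registered with the subsystem and bound to the HUD for tracking.
; Tick, the construction script and NewFunction are empty.
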(event EventTick
  (params (DeltaSeconds :type Float%20%28single-precision%29)))

(event EventBeginPlay
  (bind _returnvalue (Subsystems|GetSolarSimulationSubsystem))
  (Class|SolarSimulationSubsystem|StartRecording _returnvalue)
  (bind _returnvalue_2 (UserInterface|CreateWidget "/Game/UI/WBP_SolarHUD.WBP_SolarHUD_C" (Game|GetPlayerController 0)))
  (bind _output_get (Variables|Default|SetHUD_Widget _returnvalue_2))
  (UserInterface|Viewport|AddtoViewport _output_get 0)
  (bind _returnvalue_3 (Game|SpawnActorfromClass "/Game/Blueprints/BP_SolarPanelActor.BP_SolarPanelActor_C" (Math|Transform|MakeTransform "0.000000,0.000000,100.000000") "Undefined" "MultiplyWithRoot" 0 0))
  (bind _output_get_2 (Variables|Default|SetSolarPanel _returnvalue_3))
  (Class|SolarSimulationSubsystem|RegisterPanel _returnvalue _output_get_2)
  (Class|SolarHUDWidget|SetTrackedPanelandBind _output_get _output_get_2))

(fn ConstructionScript)

(fn NewFunction)